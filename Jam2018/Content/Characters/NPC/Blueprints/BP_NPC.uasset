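; NPC Blueprint that sets up its facial features by swapping static meshes on Nose and RightEye components.
; SetCharacteristic uses a characteristic ID to pick the component and a type ID to index that feature's mesh array.
; BeginPlay applies three hardcoded choices; IDs 0 and 2 both target the Nose, so the last call overrides the first.
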(event `self.ReceiveBeginPlay`
  (`self.SetCharacteristic` 0)
  (`self.SetCharacteristic` 1 1)
  (`self.SetCharacteristic` 2 2))

(fn `SetCharacteristic`
  (params (charID :type Integer) (typeID :type Integer))
  (switch `int` charID
    (:`0`
      (`StaticMeshComponent.SetStaticMesh` (`self.Nose`) (`|GetArrayItem` (`self.NoseMeshes`) typeID)))
    (:`1`
      (`StaticMeshComponent.SetStaticMesh` (`self.Right Eye`) (`|GetArrayItem` (`self.RightEyeMeshes`) typeID)))
    (:`2`
      (`StaticMeshComponent.SetStaticMesh` (`self.Nose`) (`|GetArrayItem` (`self.NoseMeshes`) typeID))))
  (return))

(fn `UserConstructionScript`)