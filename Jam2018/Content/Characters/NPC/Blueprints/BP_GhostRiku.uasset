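; BP_GhostRiku is a ghost NPC character Blueprint with a customizable modular appearance.
; SetCharacteristic takes a part ID and a type index, then swaps the upper, middle or lower face mesh, the neck mesh, or the first body material.
; Each option comes from a per-part array indexed directly by type.
; The event graph and construction script add no logic of their own.
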(fn `SetCharacteristic`
  (params (CharID :type Integer) (TypeId :type Integer))
  (switch `int` CharID
    (:`0`
      (`StaticMeshComponent.SetStaticMesh` (`self.CaraArriba`) (`|GetArrayItem` (`self.CaraArribaMeshes`) TypeId)))
    (:`1`
      (`StaticMeshComponent.SetStaticMesh` (`self.CaraCentro`) (`|GetArrayItem` (`self.CaraCentroMeshes`) TypeId)))
    (:`2`
      (`StaticMeshComponent.SetStaticMesh` (`self.CaraAbajo`) (`|GetArrayItem` (`self.CaraAbajoMeshes`) TypeId)))
    (:`3`
      (`StaticMeshComponent.SetStaticMesh` (`self.Cuello`) (`|GetArrayItem` (`self.CuelloMeshes`) TypeId)))
    (:`4`
      (`PrimitiveComponent.SetMaterial` (`self.Body`) 0 (`|GetArrayItem` (`self.Materiales`) TypeId))))
  (return))

(fn `UserConstructionScript`
  (`parent.UserConstructionScript`))